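; PlatformConstructor builds a WorldWidth by WorldHeight wall of platforms in the Y-Z plane, then serves as the game-end trigger.
; Each Tick it teleports to the next cell and spawns one platform, adding border duds at row wraps.
; Weighted randomness favours DudPlatform over Pattern, Random and Trigger types; pattern timings are randomised and the last cell is always a dud.
; Once built, Sphere overlap pauses the game and shows GameEndScreen.
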(event `self.ReceiveBeginPlay`
  (`self.K2_SetActorLocation` (0.0 -10.0 -24.0)))

(event `self.ReceiveTick`
  (params (DeltaSeconds :type "Float (single-precision)"))
  (bind (_returnvalue_x _returnvalue_y _returnvalue_z) (`KismetMathLibrary.BreakVector` (`self.K2_GetActorLocation`)))
  (bind (_returnvalue_x_2 _returnvalue_y_2 _returnvalue_z_2) (`KismetMathLibrary.BreakVector` (`self.K2_GetActorLocation`)))
  (bind _i (`self.i`))
  (bind _returnvalue (+ (`self.K2_GetActorLocation`) (50.0 0.0 0.0)))
  (if (< (`self.Constructed`) (* (`self.World Width`) (`self.World Height`)))
    (if (!= (mod (`self.Constructed`) (`self.World Width`)) 0.0)
      (`self.K2_SetActorLocation` (+ (`self.K2_GetActorLocation`) (0.0 50.0 0.0)) false true)
      (else
        (`|SpawnActorFromClass` "/Game/Blueprints/DudPlatform.DudPlatform_C" (`KismetMathLibrary.MakeTransform` (+ (`self.K2_GetActorLocation`) (0.0 50.0 0.0))) "Undefined" "OverrideRootScale" null null)
        (`self.K2_SetActorLocation` (`KismetMathLibrary.MakeVector` _returnvalue_x (- _returnvalue_y (* (- (`self.World Width`) 1.0) 50.0)) (+ _returnvalue_z 50.0)) false true)
        (`|SpawnActorFromClass` "/Game/Blueprints/DudPlatform.DudPlatform_C" (`KismetMathLibrary.MakeTransform` (+ (`self.K2_GetActorLocation`) (0.0 0.0 -50.0))) "Undefined" "OverrideRootScale" null null)))
    (bind _output_get (set `self.Rng` (`KismetMathLibrary.RandomFloatInRange` 1.0 15.0)))
    (if (== (`self.Constructed`) (- (* (`self.World Width`) (`self.World Height`)) 1.0))
      (`|SpawnActorFromClass` "/Game/Blueprints/DudPlatform.DudPlatform_C" (`KismetMathLibrary.MakeTransform` _returnvalue) "Undefined" "OverrideRootScale" null null :!label _label)
      (elif (< _output_get 12.0)
        (goto _label)
        (elif (< _output_get 13.0)
          (bind _returnvalue_2 (`|SpawnActorFromClass` "/Game/Blueprints/PatternPlatform.PatternPlatform_C" (`KismetMathLibrary.MakeTransform` _returnvalue) "Undefined" "OverrideRootScale" null null))
          (set `/Game/Blueprints/PatternPlatform.OpenFor` (`KismetMathLibrary.RandomFloatInRange` 1.0 10.0) _returnvalue_2)
          (set `/Game/Blueprints/PatternPlatform.ClosedFor` (`KismetMathLibrary.RandomFloatInRange` 1.0 10.0) _returnvalue_2)
          (elif (< _output_get 14.0)
            (`|SpawnActorFromClass` "/Game/Blueprints/RandomPlatform.RandomPlatform_C" (`KismetMathLibrary.MakeTransform` _returnvalue) "Undefined" "OverrideRootScale" null null)
            (else
              (`|SpawnActorFromClass` "/Game/Blueprints/TriggerPlatform.TriggerPlatform_C" (`KismetMathLibrary.MakeTransform` _returnvalue) "Undefined" "OverrideRootScale" null null))))))
    (set `self.Constructed` (+ (`self.Constructed`) 1.0))
    (else
      (while (< _i 0)
        (`|SpawnActorFromClass` "/Game/Blueprints/DudPlatform.DudPlatform_C" (`KismetMathLibrary.MakeTransform` (+ (`self.K2_GetActorLocation`) (`KismetMathLibrary.MakeVector` 0.0 50.0 (+ (* _i 50) _returnvalue_z_2)))) "Undefined" "OverrideRootScale" null null)
        (set `self.i` (+ (`self.i`) 1))))))

(event `self.Sphere.OnComponentBeginOverlap`
  (params (OverlappedComponent :type "PrimitiveComponent Object Reference") (OtherActor :type "Actor Object Reference") (OtherComp :type "PrimitiveComponent Object Reference") (OtherBodyIndex :type Integer) (bFromSweep :type Boolean) (SweepResult :type "HitResult Structure (by ref)"))
  (bind _returnvalue (`GameplayStatics.GetPlayerController` 0))
  (if (== (`self.Constructed`) (* (`self.World Width`) (`self.World Height`)))
    (`KismetSystemLibrary.Delay` 0.2)
    (`GameplayStatics.SetGamePaused` true)
    (bind _returnvalue_2 (`|CreateWidget` "/Game/Blueprints/GameEndScreen.GameEndScreen_C"))
    (`UserWidget.AddToPlayerScreen` _returnvalue_2 0)
    (`Widget.SetVisibility` _returnvalue_2 "Visible")
    (`WidgetBlueprintLibrary.SetInputMode_UIOnlyEx` _returnvalue null)
    (set `PlayerController.bShowMouseCursor` true _returnvalue)))

(fn `UserConstructionScript`)