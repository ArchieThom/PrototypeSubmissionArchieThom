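; Enemy1 is an enemy character Blueprint that chases the player and can be knocked back.
; Tick issues AIMoveTo toward the player pawn while Chasing is true and Stunned is false.
; Knockback calls StunnedEvent, which halts movement and pauses Chasing for two seconds, then launches the enemy along the TopDownCharacter's forward vector.
; Stunned is only read in this graph, so the stun works through Chasing.
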(event `Knockback`
  (`self.Stunned Event`)
  (bind _astop_down_character (cast `/Game/Blueprints/TopDownCharacter` (`GameplayStatics.GetPlayerPawn` 0)))
  (`self.LaunchCharacter` (* (`/Game/Blueprints/TopDownCharacter.ForwardVector` _astop_down_character) 1000.0)))

(event `Stunned Event`
  (`MovementComponent.StopMovementImmediately` (`self.CharacterMovement`))
  (set `self.Chasing` false)
  (`KismetSystemLibrary.Delay` 2.0)
  (set `self.Chasing` true))

(event `self.ReceiveTick`
  (params (DeltaSeconds :type "Float (single-precision)"))
  (if (and (`self.Chasing`) (not (`self.Stunned`)))
    (`|AIMoveTo` self (0.0 0.0 0.0) (`GameplayStatics.GetPlayerPawn` 0))))

(fn `UserConstructionScript`)