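; Enemy1 is a melee enemy character that chases the player pawn and trades knockback with the TopDownCharacter.
; While Chasing is set, Tick issues AIMoveTo toward the player.
; Capsule hits knock the player along the enemy's forward vector, then briefly pause the chase.
; Knockback starts a longer stun, launches the enemy along the player's facing, subtracts health and destroys it at zero; AttackingEvent is an unfinished stub.
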(event `Knockback`
  (params (PlayerStrength :type Integer))
  (bind _basehealth (`self.BaseHealth`))
  (`self.Stunned Event`)
  (bind _astop_down_character (cast `/Game/Blueprints/TopDownCharacter` (`GameplayStatics.GetPlayerPawn` 0)))
  (`self.LaunchCharacter` (* (`/Game/Blueprints/TopDownCharacter.ForwardVector` _astop_down_character) 1000.0))
  (set `self.BaseHealth` (- _basehealth PlayerStrength))
  (if (<= _basehealth 0)
    (`self.K2_DestroyActor`)))

(event `Stunned Event`
  (`MovementComponent.StopMovementImmediately` (`self.CharacterMovement`))
  (set `self.Chasing` false)
  (`KismetSystemLibrary.Delay` 2.0)
  (set `self.Chasing` true))

(event `self.ReceiveTick`
  (params (DeltaSeconds :type "Float (single-precision)"))
  (if (`self.Chasing`)
    (`|AIMoveTo` self (0.0 0.0 0.0) (`GameplayStatics.GetPlayerPawn` 0))))

(event `Attacking Event`
  (cast `/Game/Blueprints/TopDownCharacter` (`GameplayStatics.GetPlayerPawn` 0)))

(event `self.CapsuleComponent.OnComponentHit`
  (params (HitComponent :type "PrimitiveComponent Object Reference") (OtherActor :type "Actor Object Reference") (OtherComp :type "PrimitiveComponent Object Reference") (NormalImpulse :type "Vector Structure") (Hit :type "HitResult Structure (by ref)"))
  (bind _astop_down_character (cast `/Game/Blueprints/TopDownCharacter` OtherActor))
  (`/Game/Blueprints/TopDownCharacter.Player Knockback` _astop_down_character (`self.GetActorForwardVector`))
  (`self.Attack Cooldown`))

(event `Attack Cooldown`
  (`MovementComponent.StopMovementImmediately` (`self.CharacterMovement`))
  (set `self.Chasing` false)
  (`KismetSystemLibrary.Delay` 0.75)
  (set `self.Chasing` true))

(fn `UserConstructionScript`)