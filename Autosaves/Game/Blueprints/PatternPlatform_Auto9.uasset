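; PatternPlatform is a platform actor that slides out and in along world X on a repeating timed pattern.
; From BeginPlay, the In and Out events call each other after ClosedFor and OpenFor delays, toggling the Out flag.
; Tick reads that flag and sweeps the actor one unit per frame toward hard-coded world X limits, so speed depends on frame rate.
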(event `self.ReceiveBeginPlay`
  (`self.In`))

(event `Out`
  (set `self.Out?` true)
  (`KismetSystemLibrary.Delay` (`self.OpenFor`))
  (`self.In`))

(event `In`
  (set `self.Out?` false)
  (`KismetSystemLibrary.Delay` (`self.ClosedFor`))
  (`self.Out`))

(event `self.ReceiveTick`
  (params (DeltaSeconds :type "Float (single-precision)"))
  (bind _returnvalue (`self.K2_GetActorLocation`))
  (bind _returnvalue_x (`KismetMathLibrary.BreakVector` (`self.K2_GetActorLocation`)))
  (if (`self.Out?`)
    (if (>= _returnvalue_x -6.0)
      (`self.K2_SetActorLocation` (- _returnvalue (1.0 0.0 0.0)) true))
    (elif (<= _returnvalue_x 59.0)
      (`self.K2_SetActorLocation` (+ _returnvalue (1.0 0.0 0.0)) true))))

(fn `UserConstructionScript`)