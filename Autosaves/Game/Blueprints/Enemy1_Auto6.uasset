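; Enemy character Blueprint that chases the player pawn with AI MoveTo, reissued every Tick while Chasing is true.
; AttackCooldown halts movement and clears Chasing for a short delay before resuming the chase.
; Knockback, stun, attack and hit events are empty.
; Logic for a longer pause and for launching along the player's forward vector, subtracting PlayerStrength from health and destroying the enemy is present but disconnected, so it never runs.
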(event `Knockback`
  (params (PlayerStrength :type Integer)))

(event `Stunned Event`)

(event `self.ReceiveTick`
  (params (DeltaSeconds :type "Float (single-precision)"))
  (if (`self.Chasing`)
    (`|AIMoveTo` self (0.0 0.0 0.0) (`GameplayStatics.GetPlayerPawn` 0))))

(event `Attacking Event`)

(event `self.CapsuleComponent.OnComponentHit`
  (params (HitComponent :type "PrimitiveComponent Object Reference") (OtherActor :type "Actor Object Reference") (OtherComp :type "PrimitiveComponent Object Reference") (NormalImpulse :type "Vector Structure") (Hit :type "HitResult Structure (by ref)")))

(event `Attack Cooldown`
  (`MovementComponent.StopMovementImmediately` (`self.CharacterMovement`))
  (set `self.Chasing` false)
  (`KismetSystemLibrary.Delay` 0.75)
  (set `self.Chasing` true))

(fn `UserConstructionScript`)