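; TriggerPlatform is an actor that slides along the world X axis while a Player-tagged actor is inside its sphere, and slides back when that actor leaves.
; Sphere overlap events set an Out flag, which Tick reads to teleport the actor in fixed, frame-rate-dependent steps between hard-coded world X limits.
; An older swept-move version with a timed collision toggle remains disconnected and never runs.
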(event `self.Sphere.OnComponentBeginOverlap`
  (params (OverlappedComponent :type "PrimitiveComponent Object Reference") (OtherActor :type "Actor Object Reference") (OtherComp :type "PrimitiveComponent Object Reference") (OtherBodyIndex :type Integer) (bFromSweep :type Boolean) (SweepResult :type "HitResult Structure (by ref)"))
  (if (`self.ActorHasTag` OtherActor "Player")
    (set `self.Out?` true)))

(event `self.Sphere.OnComponentEndOverlap`
  (params (OverlappedComponent :type "PrimitiveComponent Object Reference") (OtherActor :type "Actor Object Reference") (OtherComp :type "PrimitiveComponent Object Reference") (OtherBodyIndex :type Integer))
  (if (`self.ActorHasTag` OtherActor "Player")
    (set `self.Out?` false)))

(event `self.ReceiveTick`
  (params (DeltaSeconds :type "Float (single-precision)"))
  (bind _returnvalue (`self.K2_GetActorLocation`))
  (bind _returnvalue_x (`KismetMathLibrary.BreakVector` (`self.K2_GetActorLocation`)))
  (if (`self.Out?`)
    (if (>= _returnvalue_x -3.0)
      (`self.K2_SetActorLocation` (- _returnvalue (2.0 0.0 0.0)) false true))
    (elif (<= _returnvalue_x 49.0)
      (`self.K2_SetActorLocation` (+ _returnvalue (2.0 0.0 0.0)) false true))))

(fn `UserConstructionScript`)