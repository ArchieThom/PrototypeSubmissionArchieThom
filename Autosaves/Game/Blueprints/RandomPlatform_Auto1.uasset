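; RandomPlatform is an actor that slides in and out along world X at random intervals, flashing as a warning before it switches back.
; Out and In events call each other through random Delays, setting the Out flag and briefly swapping Cube1 to the Flashing material before In.
; Tick reads the flag and sweeps the actor one unit per frame toward fixed absolute X limits, without delta-time scaling.
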(event `self.ReceiveBeginPlay`
  (`self.In`)
  (`PrimitiveComponent.SetMaterial` (`self.Cube1`) 0 "/Game/Blueprints/Cube.Cube"))

(event `Out`
  (set `self.Out?` true)
  (`KismetSystemLibrary.Delay` (`KismetMathLibrary.RandomFloatInRange` 1.0 10.0))
  (`PrimitiveComponent.SetMaterial` (`self.Cube1`) 0 "/Game/Blueprints/Flashing.Flashing")
  (`KismetSystemLibrary.Delay` 2.5)
  (`PrimitiveComponent.SetMaterial` (`self.Cube1`) 0 "/Game/Blueprints/Cube.Cube")
  (`self.In`))

(event `In`
  (set `self.Out?` false)
  (`KismetSystemLibrary.Delay` (`KismetMathLibrary.RandomFloatInRange` 0.1 4.0))
  (`self.Out`))

(event `self.ReceiveTick`
  (params (DeltaSeconds :type "Float (single-precision)"))
  (bind _returnvalue (`self.K2_GetActorLocation`))
  (bind _returnvalue_x (`KismetMathLibrary.BreakVector` (`self.K2_GetActorLocation`)))
  (if (`self.Out?`)
    (if (>= _returnvalue_x -3.0)
      (`self.K2_SetActorLocation` (- _returnvalue (1.0 0.0 0.0)) true))
    (elif (<= _returnvalue_x 49.0)
      (`self.K2_SetActorLocation` (+ _returnvalue (1.0 0.0 0.0)) true))))

(fn `UserConstructionScript`)