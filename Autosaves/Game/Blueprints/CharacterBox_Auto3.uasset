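; Player character Blueprint for a box character that moves by charged hops along the Y axis.
; Holding the Jump axis builds vertical launch power up to a cap, and releasing Space launches the character.
; Horizontal input only moves it while airborne, and any capsule hit clears the jumping state and resets the power.
; Unconnected leftover nodes cover a debug trace, timer, and spring-compression animation of the body, foot and spring parts.
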(event `self.ReceiveTick`
  (params (DeltaSeconds :type "Float (single-precision)")))

(event `self.ReceiveBeginPlay`
  ;[1 1 1] Movement
  (set `self.Speed` 2.0)
  (set `CharacterMovementComponent.AirControl` 0.2 (`self.CharacterMovement`))
  (set `self.Score` 0))

(event `InputAxis|Horizontal`
  (params (AxisValue :type "Float (single-precision)"))
  ;[1 1 1] Movement
  (if (`self.Jumping`)
    (`self.AddMovementInput` (`KismetMathLibrary.MakeVector` 0.0 (`self.Speed`)) AxisValue)))

(event `self.CapsuleComponent.OnComponentHit`
  (params (HitComponent :type "PrimitiveComponent Object Reference") (OtherActor :type "Actor Object Reference") (OtherComp :type "PrimitiveComponent Object Reference") (NormalImpulse :type "Vector Structure") (Hit :type "HitResult Structure (by ref)"))
  (set `self.Jumping` false)
  (set `self.LaunchPowerV2` (0.0 0.0 1.0)))

(event `InputAxis|Jump`
  (params (AxisValue :type "Float (single-precision)"))
  (bind (_launchpowerv2_x _launchpowerv2_y _launchpowerv2_z) (`KismetMathLibrary.BreakVector` (`self.LaunchPowerV2`)))
  ;[1 1 1] Jumping (top = in the air; bottom = on the ground)
  (if (> AxisValue 0.0)
    (if (< _launchpowerv2_z 800.0)
      (set `self.LaunchPowerV2` (+ (`self.LaunchPowerV2`) (0.0 0.0 16.0)))
      (if (`self.Jumping`)
        _))))

(event `Key|SpaceBar`
  (params (Key :type "Key Structure"))
  ;[1 1 1] OnJump (release)
  (:`Released`
    (if (not (`self.Jumping`))
      (set `self.Jumping` true)
      (`self.LaunchCharacter` (`self.LaunchPowerV2`))
      (set `self.LaunchPowerV2` (0.0 0.0 1.0)))))

(fn `UserConstructionScript`)