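; CubeCharacter is a physics-driven player character with a chargeable jump, pinned to a fixed X plane for side-on movement.
; Holding Jump builds capped launch power; releasing Space enables capsule physics and applies it as upward force, with horizontal input steering only while jumping.
; Capsule hits, or two offset downward traces enabled shortly after takeoff, clear the jumping state.
; Tick also counts a seconds timer through a Delay.
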(event `self.ReceiveTick`
  (params (DeltaSeconds :type "Float (single-precision)"))
  (bind (_returnvalue_x _returnvalue_y _returnvalue_z) (`KismetMathLibrary.BreakVector` (`self.K2_GetActorLocation`)))
  (`self.K2_SetActorLocation` (`KismetMathLibrary.MakeVector` -1.0 _returnvalue_y _returnvalue_z))
  (`KismetSystemLibrary.Delay` 1.0)
  (set `self.Timer` (+ (`self.Timer`) 1.0)))

(event `self.ReceiveBeginPlay`
  ;[1 1 1] Movement
  (set `self.Speed` 16000.0)
  (set `CharacterMovementComponent.AirControl` 0.2 (`self.CharacterMovement`))
  (set `self.Score` 0))

(event `InputAxis|Horizontal`
  (params (AxisValue :type "Float (single-precision)"))
  (bind _returnvalue (`self.K2_GetActorLocation`))
  ;[1 1 1] Movement
  (if (`self.Jumping`)
    (`PrimitiveComponent.AddForce` (`self.CapsuleComponent`) (`KismetMathLibrary.MakeVector` 0.0 (* AxisValue (`self.Speed`))) "None" false)
    (if (`self.GroundChecking`)
      (bind (_outhit _returnvalue_2) (`KismetSystemLibrary.LineTraceSingle` :`Start` (+ _returnvalue (0.0 25.0 0.0)) :`End` (+ _returnvalue (0.0 25.0 -30.0)) :`TraceChannel` "TraceTypeQuery1" :`DrawDebugType` "Persistent"))
      (bind (_outhit_2 _returnvalue_3) (`KismetSystemLibrary.LineTraceSingle` :`Start` (+ _returnvalue (0.0 -25.0 0.0)) :`End` (+ _returnvalue (0.0 -25.0 -30.0)) :`TraceChannel` "TraceTypeQuery1" :`DrawDebugType` "Persistent"))
      (if (or _returnvalue_3 _returnvalue_2)
        (set `self.Jumping` false)
        (set `self.GroundChecking` false)))))

(event `self.CapsuleComponent.OnComponentHit`
  (params (HitComponent :type "PrimitiveComponent Object Reference") (OtherActor :type "Actor Object Reference") (OtherComp :type "PrimitiveComponent Object Reference") (NormalImpulse :type "Vector Structure") (Hit :type "HitResult Structure (by ref)"))
  (set `self.Jumping` false)
  (set `self.LaunchPowerV2` (0.0 0.0 1.0)))

(event `InputAxis|Jump`
  (params (AxisValue :type "Float (single-precision)"))
  (bind (_launchpowerv2_x _launchpowerv2_y _launchpowerv2_z) (`KismetMathLibrary.BreakVector` (`self.LaunchPowerV2`)))
  ;[1 1 1] Jumping (top = in the air; bottom = on the ground)
  (if (> AxisValue 0.0)
    (if (< _launchpowerv2_z 7000.0)
      (set `self.LaunchPowerV2` (+ (`self.LaunchPowerV2`) (0.0 0.0 100.0)))
      (if (`self.Jumping`)
        _))))

(event `Key|SpaceBar`
  (params (Key :type "Key Structure"))
  (bind _capsulecomponent (`self.CapsuleComponent`))
  ;[1 1 1] OnJump (release)
  (:`Released`
    (set `self.Charging` false)
    (if (not (`self.Jumping`))
      (set `self.Jumping` true)
      (`PrimitiveComponent.SetSimulatePhysics` _capsulecomponent true)
      (`KismetSystemLibrary.DelayUntilNextTick`)
      (`PrimitiveComponent.AddForce` _capsulecomponent (* (`self.LaunchPowerV2`) 10) "None" true)
      (set `self.LaunchPowerV2` (0.0 0.0 100.0))
      (`KismetSystemLibrary.Delay` 0.2)
      (set `self.GroundChecking` true))))

(fn `UserConstructionScript`)